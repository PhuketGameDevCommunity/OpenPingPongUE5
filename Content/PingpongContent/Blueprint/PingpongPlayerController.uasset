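; Player controller for a Pingpong game that tracks movement control values for two players in a single controller.
; Each Tick runs both movement graphs, which scale that player's control input by speed and delta time, accumulate it, and clamp it to a symmetric range.
; Player 1's value is printed every frame; applying either value to a paddle or pawn happens outside this Blueprint.
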(event `self.ReceiveTick`
  (params (DeltaSeconds :type "Float (single-precision)"))
  (`self.Player1Movement` DeltaSeconds
    (:`OutExec`
      (`self.Player2Movement` DeltaSeconds
        (:`OutExec`
          (`KismetSystemLibrary.PrintString` (`KismetStringLibrary.Conv_DoubleToString` (`self.Player1ControlValue`))))))))

(fn `UserConstructionScript`)