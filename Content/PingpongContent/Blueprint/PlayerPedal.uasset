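; PlayerPedal is a player paddle actor for a pingpong game, assigned to player 1 or 2 through PlayerNumber.
; Each tick it reads that player's control value from the first PingpongPlayerController, so one controller drives both players.
; It treats the value as a percentage of the controller's movement range and sets the paddle's X position directly, without sweep, keeping Y and Z unchanged.
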(event `self.ReceiveTick`
  (params (DeltaSeconds :type "Float (single-precision)"))
  (bind (_x _y _z) (`KismetMathLibrary.BreakVector3f` (`self.K2_GetActorLocation`)))
  (bind (_x_2 _y_2 _z_2) (`KismetMathLibrary.BreakVector3f` (`self.K2_GetActorLocation`)))
  (bind _aspingpong_player_controller (cast `/Game/PingpongContent/Blueprint/PingpongPlayerController` (`GameplayStatics.GetPlayerController` 0)))
  (if (== (`self.PlayerNumber`) 1)
    (bind _movementpositionrange (`/Game/PingpongContent/Blueprint/PingpongPlayerController.MovementPositionRange` _aspingpong_player_controller))
    (`self.K2_SetActorLocation` (`KismetMathLibrary.MakeVector` (* _movementpositionrange (/ (`/Game/PingpongContent/Blueprint/PingpongPlayerController.Player1ControlValue` _aspingpong_player_controller) 100.0)) _y_2 _z_2))
    (elif (== (`self.PlayerNumber`) 2)
      (`self.K2_SetActorLocation` (`KismetMathLibrary.MakeVector` (* _movementpositionrange (/ (`/Game/PingpongContent/Blueprint/PingpongPlayerController.Player2ControlValue` _aspingpong_player_controller) 100.0)) _y _z)))))

(fn `UserConstructionScript`)